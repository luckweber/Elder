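; BP_FireBolt is a fire bolt actor in Elyn's fire abilities that explodes when it stops moving.
; Shortly after BeginPlay it sets FireEffect's collision to query-only.
; Each Tick compares its location with the previous frame's; at or below MinDistancePerFrame it spawns a fire hit sound and effect, then destroys itself.
; The file itself contains no movement or damage logic, and its overlap event is unused.
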(event EventBeginPlay
  (Utilities|FlowControl|Delay 0.1)
  (bind _fireeffect (Variables|Default|GetFireEffect)
    (:then
      (Collision|SetCollisionEnabled _fireeffect "QueryOnly"))
    (:else)))

(event Collision|EventActorBeginOverlap
  (params (OtherActor :type Actor%20Object%20Reference)))

(event EventTick
  (params (DeltaSeconds :type Float%20%28single-precision%29))
  (CallFunction|MakeGoKaboomifNoMove))

(fn ConstructionScript)

(fn MakeGoKaboomifNoMove
  (Variables|Default|SetLocationLastFrame (Variables|Default|GetLocationThisFrame))
  (Variables|Default|SetLocationThisFrame (Transformation|GetActorLocation))
  (if (<= (Math|Vector|VectorLength (- (Variables|Default|GetLocationThisFrame) (Variables|Default|GetLocationLastFrame))) (Variables|Default|GetMinDistancePerFrame))
    (Audio|SpawnSoundatLocation "/Game/FantasyBundle1/cues/Ultimate_Magic_Spells/Target_Hits/Target_Hit_-_Fire__1__Cue.Target_Hit_-_Fire__1__Cue" (Variables|Default|GetLocationThisFrame) "0, 0, 0" 1.0 1.0 0.0 0 0)
    (Niagara|SpawnSystematLocation "/Game/MagicKit/Particles/Fire/NS_Fire_Hit_01.NS_Fire_Hit_01" (Variables|Default|GetLocationThisFrame))
    (Actor|DestroyActor)))